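; BP_Enemy is an enemy that flies in a straight line and destroys the player on contact.
; On BeginPlay, a random roll against TraceRate either aims and rotates it toward the player's current position or keeps its forward vector as the direction (방향).
; Tick moves it along that fixed direction at 이동속도 (move speed), without sweep.
; Overlapping BP_Player destroys both actors and spawns P_Explosion at the enemy's location.
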(event EventBeginPlay
  (if (<= (Math|Random|RandomFloatinRange 0.0 1.0) (Variables|Default|GetTrace%20Rate))
    (bind _returnvalue (Actor|GetActorOfClass "/Game/Blueprints/BP_Player.BP_Player_C"))
    (Utilities|IsValid _returnvalue
      (:Is%20Valid
        (bind _output_get (Variables|Default|Set방향 (Math|Vector|Normalize (- (Transformation|GetActorLocation _returnvalue) (Transformation|GetActorLocation)))))
        (Transformation|SetActorRotation (Math|Rotator|MakeRotfromXZ _output_get (Transformation|GetActorUpVector)))))
    (else
      (Variables|Default|Set방향 (Transformation|GetActorForwardVector)))))

(event Collision|EventActorBeginOverlap
  (params (OtherActor :type Actor%20Object%20Reference))
  (bind _asbp_player (Utilities|Casting|CastToBP_Player OtherActor))
  (Actor|DestroyActor _asbp_player)
  (Effects|SpawnEmitteratLocation "/Game/StarterContent/Particles/P_Explosion.P_Explosion" (Transformation|GetActorLocation))
  (Actor|DestroyActor))

(event EventTick
  (params (DeltaSeconds :type Float%20%28single-precision%29))
  (Transformation|SetActorLocation (+ (Transformation|GetActorLocation) (* (* (Variables|Default|Get방향) (Variables|Default|Get이동속도)) DeltaSeconds)) false false))

(fn ConstructionScript)